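; Tree enemy that reaches its arm toward the player inside its collision volume and drains the WillOWispCharacter's health on arm contact until death.
; Timelines drive lerped reaching with head tracking, interpolated retraction to the base, and repeated damage.
; An overlapping MagicBall diverts arm and head toward itself.
; A follow-up check then resumes pursuit if the player is moving inside the volume, otherwise starts retracting.
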(event `Get Distracted`
  (bind _returnvalue (`GameplayStatics.GetPlayerCharacter` 0))
  (bind _head (`self.Head`))
  (bind _arm (`self.Arm`))
  (bind _arm_2 (`self.Arm`))
  (bind _base (`self.Base`))
  (bind _arm_3 (`self.Arm`))
  (bind _base_2 (`self.Base`))
  ;[1 1 1] Magic Ball Interaction
  (`|ExecutionSequence`
    (:`then_0`
      ;;[1 1 1] Check if the Player is still in range and moving
      (`Timeline|Check for movement` :!via `Stop` :!label _label
        (:`Update`
          (if (`PrimitiveComponent.IsOverlappingActor` (`self.Collision`) _returnvalue)
            (if (> (`KismetMathLibrary.VSize` (`self.GetVelocity` _returnvalue)) 0.0)
              (`self.Activate`)
              (`|ExecutionSequence`
                (:`then_0`
                  (goto _label :!via `Stop`))
                (:`then_1`
                  (bind (_direction _newtrack_0) (`Timeline|SoundRetract` :!via `Stop` :!label _label_2)
                    (:`Update`
                      ;;[1 1 1] Retract
                      (`SceneComponent.K2_SetWorldLocationAndRotation` _arm_3 (`KismetMathLibrary.VInterpTo` (`SceneComponent.K2_GetComponentLocation` _arm_3) (`SceneComponent.K2_GetComponentLocation` _base_2) (`GameplayStatics.GetWorldDeltaSeconds`) _newtrack_0) (`KismetMathLibrary.RLerp` (`SceneComponent.K2_GetComponentRotation` _arm_3) (`KismetMathLibrary.MakeRotator` (+ (.roll (`KismetMathLibrary.FindLookAtRotation` (`SceneComponent.K2_GetComponentLocation` _arm_3) (`SceneComponent.K2_GetComponentLocation` _base_2))) 0.0) (+ (.pitch (`KismetMathLibrary.FindLookAtRotation` (`SceneComponent.K2_GetComponentLocation` _arm_3) (`SceneComponent.K2_GetComponentLocation` _base_2))) 90.0) (+ (.yaw (`KismetMathLibrary.FindLookAtRotation` (`SceneComponent.K2_GetComponentLocation` _arm_3) (`SceneComponent.K2_GetComponentLocation` _base_2))) 0.0)) 0.03 true) false false)))))
              (else
                (goto _label_2 :!via `PlayFromStart`)))
            (else
              (goto _label_2 :!via `PlayFromStart`))))
        (:`Finished`
          (goto _label_2 :!via `Stop`))))
    (:`then_1`
      (goto _label_2 :!via `Stop`))
    (:`then_2`
      (`Timeline|SoundReach` :!via `Stop` :!label _label_3
        (:`Update`
          (`|ExecutionSequence`
            (:`then_0`
              ;[1 1 1] Player Interaction
              (bind (_direction_2 _newtrack_0_2) (`Timeline|PlayerRetract` :!via `Stop` :!label _label_4)
                (:`Update`
                  ;;[1 1 1] Retract
                  (`SceneComponent.K2_SetWorldLocationAndRotation` _arm_2 (`KismetMathLibrary.VInterpTo` (`SceneComponent.K2_GetComponentLocation` _arm_2) (`SceneComponent.K2_GetComponentLocation` _base) (`GameplayStatics.GetWorldDeltaSeconds`) _newtrack_0_2) (`KismetMathLibrary.RLerp` (`SceneComponent.K2_GetComponentRotation` _arm_2) (`KismetMathLibrary.MakeRotator` (+ (.roll (`KismetMathLibrary.FindLookAtRotation` (`SceneComponent.K2_GetComponentLocation` _arm_2) (`SceneComponent.K2_GetComponentLocation` _base))) 0.0) (+ (.pitch (`KismetMathLibrary.FindLookAtRotation` (`SceneComponent.K2_GetComponentLocation` _arm_2) (`SceneComponent.K2_GetComponentLocation` _base))) 90.0) (+ (.yaw (`KismetMathLibrary.FindLookAtRotation` (`SceneComponent.K2_GetComponentLocation` _arm_2) (`SceneComponent.K2_GetComponentLocation` _base))) 0.0)) 0.03 true) false false))))
            (:`then_1`
              ;;[1 1 1] Reach Out
              (`SceneComponent.K2_SetWorldLocationAndRotation` _arm (`KismetMathLibrary.VLerp` (`SceneComponent.K2_GetComponentLocation` _arm) (`self.K2_GetActorLocation` (stale `self.Collision.OnComponentBeginOverlap` _asmagic_ball)) 0.015) (`KismetMathLibrary.MakeRotator` (.roll (`KismetMathLibrary.FindLookAtRotation` (`SceneComponent.K2_GetComponentLocation` _arm) (`self.K2_GetActorLocation` (stale `self.Collision.OnComponentBeginOverlap` _asmagic_ball)))) (- (.pitch (`KismetMathLibrary.FindLookAtRotation` (`SceneComponent.K2_GetComponentLocation` _arm) (`self.K2_GetActorLocation` (stale `self.Collision.OnComponentBeginOverlap` _asmagic_ball)))) 90.0) (.yaw (`KismetMathLibrary.FindLookAtRotation` (`SceneComponent.K2_GetComponentLocation` _arm) (`self.K2_GetActorLocation` (stale `self.Collision.OnComponentBeginOverlap` _asmagic_ball))))) false false)
              ;;[1 1 1] Turn Head
              (`SceneComponent.K2_SetWorldRotation` _head (`KismetMathLibrary.RLerp` (`SceneComponent.K2_GetComponentRotation` _head) (`KismetMathLibrary.FindLookAtRotation` (`SceneComponent.K2_GetComponentLocation` _head) (`self.K2_GetActorLocation` (stale `self.Collision.OnComponentBeginOverlap` _asmagic_ball))) 0.1 true) false false))
            (:`then_2`
              (goto _label_2 :!via `Stop`))))
        (:`Finished`
          (goto _label))))
    (:`then_3`
      (goto _label_3 :!via `PlayFromStart`))))

(event `self.Collision.OnComponentBeginOverlap`
  (params (OverlappedComponent :type "PrimitiveComponent Object Reference") (OtherActor :type "Actor Object Reference") (OtherComp :type "PrimitiveComponent Object Reference") (OtherBodyIndex :type Integer) (bFromSweep :type Boolean) (SweepResult :type "HitResult Structure (by ref)"))
  (bind _arm (`self.Arm`))
  (bind _head (`self.Head`))
  ;[1 1 1] Magic Ball or Player?
  (bind _asmagic_ball (cast `/Game/MagicBall` OtherActor)
    (:`then`
      (`KismetSystemLibrary.PrintString` "It hears the ball")
      (`self.Get Distracted`)
      (`|ExecutionSequence`
        (:`then_0`
          ;[1 1 1] Player Interaction
          (`Timeline|PlayerReach` :!via `Stop` :!label _label_5
            (:`Update`
              ;;[1 1 1] Reach Out
              (`SceneComponent.K2_SetWorldLocationAndRotation` _arm (`KismetMathLibrary.VLerp` (`SceneComponent.K2_GetComponentLocation` _arm) (`self.K2_GetActorLocation` (`GameplayStatics.GetPlayerCharacter` 0)) 0.015) (`KismetMathLibrary.MakeRotator` (.roll (`KismetMathLibrary.FindLookAtRotation` (`SceneComponent.K2_GetComponentLocation` _arm) (`self.K2_GetActorLocation` (`GameplayStatics.GetPlayerCharacter` 0)))) (- (.pitch (`KismetMathLibrary.FindLookAtRotation` (`SceneComponent.K2_GetComponentLocation` _arm) (`self.K2_GetActorLocation` (`GameplayStatics.GetPlayerCharacter` 0)))) 90.0) (.yaw (`KismetMathLibrary.FindLookAtRotation` (`SceneComponent.K2_GetComponentLocation` _arm) (`self.K2_GetActorLocation` (`GameplayStatics.GetPlayerCharacter` 0))))) false false)
              ;;[1 1 1] Turn Head
              (`SceneComponent.K2_SetWorldRotation` _head (`KismetMathLibrary.RLerp` (`SceneComponent.K2_GetComponentRotation` _head) (`KismetMathLibrary.FindLookAtRotation` (`SceneComponent.K2_GetComponentLocation` _head) (`self.K2_GetActorLocation` (`GameplayStatics.GetPlayerCharacter` 0))) 0.2 true) false false))))
        (:`then_1`
          (goto _label_4 :!via `Stop`))))
    (:`CastFailed`
      (if (== OtherActor (`GameplayStatics.GetPlayerCharacter` 0))
        (`self.Activate`)
        (`|ExecutionSequence`
          (:`then_0`
            (goto _label_3 :!via `Stop`))
          (:`then_1`
            (goto _label_2 :!via `Stop`)))))))

(event `self.Collision.OnComponentEndOverlap`
  (params (OverlappedComponent :type "PrimitiveComponent Object Reference") (OtherActor :type "Actor Object Reference") (OtherComp :type "PrimitiveComponent Object Reference") (OtherBodyIndex :type Integer))
  ;[1 1 1] Player Exit
  (if (== OtherActor (`GameplayStatics.GetPlayerCharacter` 0))
    (`self.Deactivate`)))

(event `Activate`
  ;[1 1 1] Player Interaction
  (`|ExecutionSequence`
    (:`then_0`
      (goto _label_4 :!via `Stop`))
    (:`then_1`
      (goto _label_5))))

(event `self.Arm.OnComponentBeginOverlap`
  (params (OverlappedComponent :type "PrimitiveComponent Object Reference") (OtherActor :type "Actor Object Reference") (OtherComp :type "PrimitiveComponent Object Reference") (OtherBodyIndex :type Integer) (bFromSweep :type Boolean) (SweepResult :type "HitResult Structure (by ref)"))
  ;[1 1 1] Touching / Hurting / Killing Player
  (bind _aswill_owisp_character (cast `/Game/WillOWispCharacter` OtherActor))
  (`Timeline|Damages` :!label _label_6
    (:`Update`
      (set `/Game/WillOWispCharacter.Health` (- (`/Game/WillOWispCharacter.Health` _aswill_owisp_character) 0.01) _aswill_owisp_character)
      (`/Game/WillOWispCharacter.Hurting` _aswill_owisp_character)
      (if (<= (`/Game/WillOWispCharacter.Health` _aswill_owisp_character) 0.0)
        (`/Game/WillOWispCharacter.Dying` _aswill_owisp_character)
        (`|ExecutionSequence`
          (:`then_0`
            (goto _label_6 :!via `Stop`))
          (:`then_1`
            (goto _label_5 :!via `Stop`))
          (:`then_2`
            (goto _label_4 :!via `PlayFromStart`)))))))

(event `Deactivate`
  ;[1 1 1] Player Interaction
  (`|ExecutionSequence`
    (:`then_0`
      (goto _label_5 :!via `Stop`))
    (:`then_1`
      (goto _label_4 :!via `PlayFromStart`))))

(event `self.Arm.OnComponentEndOverlap`
  (params (OverlappedComponent :type "PrimitiveComponent Object Reference") (OtherActor :type "Actor Object Reference") (OtherComp :type "PrimitiveComponent Object Reference") (OtherBodyIndex :type Integer))
  ;[1 1 1] Touching / Hurting / Killing Player
  (cast `/Game/WillOWispCharacter` OtherActor)
  (goto _label_6 :!via `Stop`))

(fn `UserConstructionScript`
  (`PrimitiveComponent.SetMaterial` (`self.Body`) 0 "/Game/StarterContent/Materials/M_Wood_Oak.M_Wood_Oak")
  (`PrimitiveComponent.SetMaterial` (`self.Head`) 0 "/Game/StarterContent/Materials/M_Wood_Oak.M_Wood_Oak")
  (`PrimitiveComponent.SetMaterial` (`self.Arm`) 0 "/Game/StarterContent/Materials/M_Wood_Oak.M_Wood_Oak"))